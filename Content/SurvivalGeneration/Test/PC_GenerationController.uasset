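; Test player controller that generates a chunked voxel world around the player in survival generation.
; On BeginPlay it fills a render-range grid of VoxelChank actors, stored in Map as lines.
; Tick detects chunk changes: zero X shift spawns a BP_Voxel grid, +1 destroys the first line and calls SpawnNewLine.
; SpawnNewLine is unfinished, spawning one chunk and polling IsSpawned without storing it; K spawns debug chunks.
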(event Custom|PlayerHasChangedChunkCoordinates
  (CallFunction|SpawnChuncswithRenderRange))

(event Custom|SpawnNewLine
  (bind _position (CallFunction|GetPlayerChunkCoordinates))
  (Variables|Default|SetisSpawned false)
  (Variables|Default|SetX_Index 1)
  (Variables|Default|SetY_Index -1)
  (if (< (Variables|Default|GetY_Index) 2)
    (Development|PrintString "SPAWN!")
    (Game|SpawnActorfromClass "/Script/SurvivalGame.VoxelChank" (Math|Transform|MakeTransform (Math|Vector|MakeVector (* (+ (.x _position) (Variables|Default|GetX_Index)) (Variables|WorldGen|GetChunkSizeXY)) (* (+ (.y _position) (Variables|Default|GetY_Index)) (Variables|WorldGen|GetChunkSizeXY)) 0.0) "0, 0, 0" "1,1,1") "Undefined" 0 0)
    (if (Variables|Default|GetisSpawned) :!label _label
      (Variables|Default|SetisSpawned false)
      (Math|Integer|IncrementInt (Variables|Default|GetY_Index))
      (else
        (Utilities|FlowControl|Delay 0.2)
        (goto _label)))))

(event EventBeginPlay
  (CallFunction|InitWorld))

(event EventTick
  (params (DeltaSeconds :type Float%20%28single-precision%29))
  (bind _position (CallFunction|GetPlayerChunkCoordinates))
  (bind _position_2 (CallFunction|GetPlayerChunkCoordinates))
  (if (not (and (== (.x _position) (.x (Variables|WorldGen|GetLastKnownChunkCoordinates))) (== (.y _position) (.y (Variables|WorldGen|GetLastKnownChunkCoordinates)))))
    (Variables|Default|SetX_Shift (- (.x _position) (.x (Variables|WorldGen|GetLastKnownChunkCoordinates))))
    (Variables|Default|SetY_Shift (- (.y _position) (.y (Variables|WorldGen|GetLastKnownChunkCoordinates))))
    (Variables|WorldGen|SetLastKnownChunkCoordinates (Utilities|Struct|MakeIntVector (.x _position_2) (.y _position_2) 0))
    (CallFunction|PlayerHasChangedChunkCoordinates)))

(event Input|KeyboardEvents|K
  (params (Key :type Key%20Structure :default "None"))
  (:Pressed
    (for _index (range 0 3)
      (CallFunction|SpawnChunk 1e+03 (Math|Conversions|ToFloat(Integer) (* _index 1000)) 1e+03))))

(fn ConstructionScript)

(fn SpawnChunk
  (params (ChunkCoordinatesX :type Float%20%28single-precision%29) (ChunkCoordinatesY :type Float%20%28single-precision%29) (ChunkCoordinatesZ :type Float%20%28single-precision%29))
  (Game|SpawnActorfromClass "/Script/SurvivalGame.VoxelChank" (Math|Transform|MakeTransform (Math|Vector|MakeVector ChunkCoordinatesX ChunkCoordinatesY ChunkCoordinatesZ) "0, 0, 0" "1,1,1") "Undefined" 0 0))

(fn SpawnChuncswithRenderRange
  (bind _position (CallFunction|GetPlayerChunkCoordinates))
  (bind _renderrange (Variables|WorldGen|GetRenderRange))
  (bind _map (Variables|Default|GetMap))
  (bind _renderrange_2 (Variables|WorldGen|GetRenderRange))
  (bind _output (Utilities|Array|Get(acopy) _map))
  (if (== (Variables|Default|GetX_Shift) 0)
    (for _index (range (* _renderrange -1) _renderrange)
      (LocalVariables|SetX _index)
      (for _index_2 (range (* _renderrange_2 -1) _renderrange_2)
        (LocalVariables|SetY _index_2)
        (Game|SpawnActorfromClass "/Game/SurvivalGeneration/Test/BP_Voxel.BP_Voxel_C" (Math|Transform|MakeTransform (Math|Vector|MakeVector (* (+ (.x _position) (LocalVariables|GetX)) (Variables|WorldGen|GetChunkSizeXY)) (* (+ (.y _position) (LocalVariables|GetY)) (Variables|WorldGen|GetChunkSizeXY)) 0.0) "0, 0, 0" "1,1,1") "Undefined" 0 0.0001 10 25 0)))
    (elif (== (Variables|Default|GetX_Shift) 1)
      (Development|PrintString "Hello")
      (while (> (Utilities|Array|Length (.column _output)) 0)
        (Actor|DestroyActor (Utilities|Array|Get(acopy) (.column _output)))
        (Utilities|Array|RemoveIndex (.column _output)))
      (Utilities|Array|RemoveIndex (Variables|Default|GetMap))
      (LocalVariables|SetX 1)
      (CallFunction|SpawnNewLine))))

(fn GetPlayerChunkCoordinates
  (bind _returnvalue (Game|Player|GetPlayerPawn 0))
  (bind _chunksizexy (Variables|WorldGen|GetChunkSizeXY))
  (bind _returnvalue_2 (Transformation|GetActorLocation _returnvalue))
  (bind _returnvalue_3 (/ _returnvalue_2 _chunksizexy))
  (return (Utilities|Struct|MakeIntVector (Math|Float|Round (.x _returnvalue_3)) (Math|Float|Round (.y _returnvalue_3)))))

(fn InitWorld
  (bind _position (CallFunction|GetPlayerChunkCoordinates))
  (bind _returnvalue (Transformation|GetActorLocation))
  (bind _renderrange (Variables|WorldGen|GetRenderRange))
  (bind _renderrange_2 (Variables|WorldGen|GetRenderRange))
  (bind _chunksizexy (Variables|WorldGen|GetChunkSizeXY))
  (for _index (range (* _renderrange_2 -1) _renderrange_2)
    (Utilities|Array|Clear (.column (LocalVariables|GetLine)))
    (LocalVariables|SetX _index)
    (for _index_2 (range (* _renderrange -1) _renderrange)
      (LocalVariables|SetY _index_2)
      (Math|Integer|IncrementInt (LocalVariables|GetCount)
        (:%20%20
          (bind _returnvalue_2 (Game|SpawnActorfromClass "/Script/SurvivalGame.VoxelChank" (Math|Transform|MakeTransform (Math|Vector|MakeVector (* (+ (.x _position) (LocalVariables|GetX)) (Variables|WorldGen|GetChunkSizeXY)) (* (+ (.y _position) (LocalVariables|GetY)) (Variables|WorldGen|GetChunkSizeXY)) 0.0) "0, 0, 0" "1,1,1") "Undefined" 0 0))
          (Utilities|Array|Add (.column (LocalVariables|GetLine)) _returnvalue_2))))
    (Utilities|Array|Add (Variables|Default|GetMap) (LocalVariables|GetLine)))
  (Development|PrintString (Utilities|String|ToString(Integer) (LocalVariables|GetCount)))
  (for _array_element (Variables|Default|GetMap)
    (for _array_element_2 (.column _array_element)
      (Development|PrintString (Utilities|String|ToString(Vector) (Math|Vector|MakeVector (/ (.x _returnvalue) _chunksizexy) (/ (.y _returnvalue) _chunksizexy) 0.0)) true true "(R=0.000000,G=0.660000,B=1.000000,A=1.000000)" 1e+01))))