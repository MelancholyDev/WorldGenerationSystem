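; Test voxel terrain chunk that builds a block landscape with caves from instanced static meshes in its construction script.
; It loops over a grid of columns and depth layers, offsetting each column by 2D simplex noise sampled at actor-offset coordinates.
; Below the top few layers, 3D simplex noise in chunk-local coordinates culls voxels under a threshold to carve caves.
; On BeginPlay it sets IsSpawned on the generation player controller.
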(event EventBeginPlay
  (bind _aspc_generation_controller (Utilities|Casting|CastToPC_GenerationController (Game|GetPlayerController 0)))
  (Variables|/Game/SurvivalGeneration/Test/PC_GenerationController.PC_GenerationController_C|SetisSpawned _aspc_generation_controller true))

(fn ConstructionScript
  (bind _chanksize (Variables|Default|GetChankSize))
  (bind _chanksize_2 (Variables|Default|GetChankSize))
  (for _index (range (* _chanksize -1) _chanksize)
    (LocalVariables|SetLoopX _index)
    (for _index_2 (range (* _chanksize_2 -1) _chanksize_2)
      (LocalVariables|SetLoopY _index_2)
      (for _index_3 (range (* (Variables|Default|GetDepth) -1) 0)
        (LocalVariables|SetLoopZ _index_3)
        (LocalVariables|SetPreNoiseZ (.Z (Utilities|ActorLocation (LocalVariables|GetLoopX) (LocalVariables|GetLoopY) (LocalVariables|GetLoopZ))))
        (bind _returnvalue (Class|SimplexNoiseBPLibrary|SimplexNoise2D (.X (Utilities|ActorLocation (LocalVariables|GetLoopX) (LocalVariables|GetLoopY) (LocalVariables|GetLoopZ))) (.Y (Utilities|ActorLocation (LocalVariables|GetLoopX) (LocalVariables|GetLoopY) (LocalVariables|GetLoopZ))) (Variables|Default|GetNoiseDensity)))
        (LocalVariables|SetPostNoiseZ (- (Math|Float|Floor (* (Variables|Default|GetNoiseScale) _returnvalue)) (LocalVariables|GetLoopZ)))
        (if (< (LocalVariables|GetLoopZ) -3)
          (bind _returnvalue_2 (Class|SimplexNoiseBPLibrary|SimplexNoise3D (.X (Math|Vector|BreakVector (Math|Vector|MakeVector (* (LocalVariables|GetLoopX) (Variables|Default|GetVoxelSize)) (* (LocalVariables|GetLoopY) (Variables|Default|GetVoxelSize)) (* -1 (* (LocalVariables|GetPostNoiseZ) (Variables|Default|GetVoxelSize)))))) (.Y (Math|Vector|BreakVector (Math|Vector|MakeVector (* (LocalVariables|GetLoopX) (Variables|Default|GetVoxelSize)) (* (LocalVariables|GetLoopY) (Variables|Default|GetVoxelSize)) (* -1 (* (LocalVariables|GetPostNoiseZ) (Variables|Default|GetVoxelSize)))))) (.Z (Math|Vector|BreakVector (Math|Vector|MakeVector (* (LocalVariables|GetLoopX) (Variables|Default|GetVoxelSize)) (* (LocalVariables|GetLoopY) (Variables|Default|GetVoxelSize)) (* -1 (* (LocalVariables|GetPostNoiseZ) (Variables|Default|GetVoxelSize)))))) (Variables|Default|Get3DNoiseDensity)))
          (if (not (< _returnvalue_2 (Variables|Default|Get3DThreshold)))
            (Components|InstancedStaticMesh|AddInstance (Variables|Default|GetInstancedStaticMesh) (Math|Transform|MakeTransform (Math|Vector|MakeVector (* (LocalVariables|GetLoopX) (Variables|Default|GetVoxelSize)) (* (LocalVariables|GetLoopY) (Variables|Default|GetVoxelSize)) (* -1 (* (LocalVariables|GetPostNoiseZ) (Variables|Default|GetVoxelSize)))) "0, 0, 0" "0.500000,0.500000,0.500000") :!label _label))
          (else
            (goto _label)))))))

(fn AddNoise
  (params (Noise :type Float%20%28single-precision%29) (XTransform :type Float%20%28single-precision%29) (YTransform :type Float%20%28single-precision%29))
  (Components|InstancedStaticMesh|AddInstance (Variables|Default|GetInstancedStaticMesh) (Math|Conversions|ToTransform(Vector) (Math|Vector|MakeVector XTransform YTransform (* (Math|Float|Floor (* 10 Noise)) 1e+02)))))

(fn IsVoxelEmpty
  (params (X :type Float%20%28single-precision%29) (Y :type Float%20%28single-precision%29) (Z :type Float%20%28single-precision%29))
  (bind _returnvalue (Class|SimplexNoiseBPLibrary|SimplexNoise2D X Y 1.0))
  (LocalVariables|SetFlatPerlin _returnvalue)
  (LocalVariables|SetTerrainHeight (* (Math|Float|Floor (* 10 (LocalVariables|GetFlatPerlin))) 1e+02))
  (bind _returnvalue_2 (Class|SimplexNoiseBPLibrary|SimplexNoise3D X Y Z 1.0))
  (return (or (> _returnvalue_2 (LocalVariables|GetThreshold)) (> Y (LocalVariables|GetTerrainHeight)))))