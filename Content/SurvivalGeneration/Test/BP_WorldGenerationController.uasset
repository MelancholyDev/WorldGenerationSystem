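; Debug controller for testing world generation, driven by number-key presses.
; Keys 1–4 shift the player pawn diagonally in XY at constant Z through TeleportChartacterWithShift, which wraps TeleportCharacter.
; Keys 7 and 8 print multi-octave simplex noise samples at fixed coordinates, and a second key 7 binding prints the VoxelChank actor count.
; Key 5 calls GetFullSize, and some unwired noise and teleport test nodes remain.
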(event Input|KeyboardEvents|5
  (params (Key :type Key%20Structure :default "None"))
  (:Pressed
    (Class|GenerationPlayerController|GetFullSize)))

(event Input|KeyboardEvents|7
  (params (Key :type Key%20Structure :default "None"))
  (:Pressed
    (bind _outactors (Actor|GetAllActorsOfClass "/Script/SurvivalGame.VoxelChank"))
    (Development|PrintString (Utilities|String|ToString(Integer) (Utilities|Array|Length _outactors)))))

(event Input|KeyboardEvents|1
  (params (Key :type Key%20Structure :default "None"))
  (:Pressed
    (CallFunction|TeleportChartacterwithShift 1e+03 -1e+03)))

(event Input|KeyboardEvents|2
  (params (Key :type Key%20Structure :default "None"))
  (:Pressed
    (CallFunction|TeleportChartacterwithShift 1e+03 1e+03)))

(event Input|KeyboardEvents|3
  (params (Key :type Key%20Structure :default "None"))
  (:Pressed
    (CallFunction|TeleportChartacterwithShift -1e+03 -1e+03)))

(event Input|KeyboardEvents|4
  (params (Key :type Key%20Structure :default "None"))
  (:Pressed
    (CallFunction|TeleportChartacterwithShift -1e+03 1e+03)))

(event Input|KeyboardEvents|8
  (params (Key :type Key%20Structure :default "None")))

(event Input|KeyboardEvents|7
  (params (Key :type Key%20Structure :default "None"))
  (:Pressed
    (bind _returnvalue (Class|SimplexNoiseBPLibrary|GetSimplexNoise2DEX 1.12e+04 -5.9e+03 2.3 0.6 6 2e-05 true))
    (Development|PrintString (Utilities|String|ToString(Float) _returnvalue))))

(event Input|KeyboardEvents|8
  (params (Key :type Key%20Structure :default "None"))
  (:Pressed
    (bind _returnvalue (Class|SimplexNoiseBPLibrary|GetSimplexNoise2DEX 1.12e+04 -6e+03 2.3 0.6 6 2e-05 true))
    (Development|PrintString (Utilities|String|ToString(Float) _returnvalue))))

(fn ConstructionScript)

(fn TeleportCharacter
  (params (X :type Float%20%28single-precision%29) (Y :type Float%20%28single-precision%29) (Z :type Float%20%28single-precision%29))
  (Transformation|SetActorLocation (Game|Player|GetPlayerPawn 0) (Math|Vector|MakeVector X Y Z) false false))

(fn TeleportChartacterwithShift
  (params (XShift :type Float%20%28single-precision%29) (YShift :type Float%20%28single-precision%29))
  (bind _returnvalue (Game|Player|GetPlayerPawn 0))
  (bind _returnvalue_2 (Transformation|GetActorLocation _returnvalue))
  (CallFunction|TeleportCharacter (+ (.x _returnvalue_2) XShift) (+ YShift (.y _returnvalue_2)) (.z _returnvalue_2)))