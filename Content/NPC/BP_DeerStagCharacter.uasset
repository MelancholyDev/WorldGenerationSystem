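; Stag deer NPC that, when flagged as leader, spawns and leads a herd shortly after BeginPlay.
; The herd randomly mixes stags and does at reachable nearby points with varied yaw and scale, each given a default controller and Leader reference.
; AlertHerd and StopAlert toggle the leader's blackboard alert keys.
; They also set whether a lion AI controller can see the player, clearing it after a delay.
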(event Custom|SpawnHerd
  (bind _returnvalue (Math|Random|RandomFloatinRange 0.5 0.9))
  (bind _self self)
  (for _index (range 0 (Variables|Default|GetHerdSize))
    (bind _returnvalue_2 (Game|SpawnActorfromClass (Utilities|Select :Index (Math|Random|RandomIntegerinRange 0 1) :Option%200 "BP_DeerStagCharacter_C" :Option%201 "/Game/NPC/BP_DeerDoeCharacter.BP_DeerDoeCharacter_C") (Math|Transform|MakeTransform (.RandomLocation (AI|Navigation|GetRandomReachablePointinRadius (Transformation|GetActorLocation) 1e+03 0 0)) (Math|Rotator|MakeRotator 0.0 0.0 (Math|Random|RandomFloatinRange 0.0 3.6e+02)) (Math|Vector|MakeVector _returnvalue _returnvalue _returnvalue)) "AdjustIfPossibleButDontSpawnIfColliding" 0 0))
    (Utilities|IsValid _returnvalue_2
      (:Is%20Valid
        (Utilities|Array|Add (Variables|Default|GetHerd) _returnvalue_2))))
  (for _array_element (Variables|Default|GetHerd)
    (bind _asbp_deer_stag_character (Utilities|Casting|CastToBP_DeerStagCharacter _array_element)
      (:then
        (Pawn|SpawnDefaultController _asbp_deer_stag_character)
        (Variables|BP_DeerStagCharacter_C|SetLeader _asbp_deer_stag_character _self))
      (:CastFailed
        (Pawn|SpawnDefaultController (.AsBP%20Deer%20Doe%20Character (Utilities|Casting|CastToBP_DeerDoeCharacter _array_element)))
        (Variables|/Game/NPC/BP_DeerDoeCharacter.BP_DeerDoeCharacter_C|SetLeader (.AsBP%20Deer%20Doe%20Character (Utilities|Casting|CastToBP_DeerDoeCharacter _array_element)) _self)))))

(event Custom|StopAlert
  (if (Variables|Default|GetIsLeader?)
    (Variables|Default|SetIsAlert? false)
    (AI|Components|Blackboard|SetValueasBool (AI|GetBlackboard (Variables|Default|GetLeader)) (Variables|Default|GetKeyAlert) false)
    (AI|Components|Blackboard|SetValueasBool (AI|GetBlackboard (Variables|Default|GetLeader)) (Variables|Default|GetKeyLeader) false)
    (Utilities|FlowControl|Delay 5.0)
    (bind _returnvalue (Actor|GetActorOfClass "/Game/NPC/BP_BT_LionController.BP_BT_LionController_C"))
    (Default|SetCanSeePlayer? _returnvalue false (.AsFirst%20Person%20Character (Utilities|Casting|CastToFirstPersonCharacter (Game|GetPlayerCharacter 0))))))

(event Custom|Alert%20Herd
  (if (Variables|Default|GetIsLeader?)
    (Variables|Default|SetIsAlert? true)
    (AI|Components|Blackboard|SetValueasBool (AI|GetBlackboard (Variables|Default|GetLeader)) (Variables|Default|GetKeyAlert) true)
    (AI|Components|Blackboard|SetValueasBool (AI|GetBlackboard (Variables|Default|GetLeader)) (Variables|Default|GetKeyLeader) true)
    (bind _returnvalue (Actor|GetActorOfClass "/Game/NPC/BP_BT_LionController.BP_BT_LionController_C"))
    (Default|SetCanSeePlayer? _returnvalue true (.AsFirst%20Person%20Character (Utilities|Casting|CastToFirstPersonCharacter (Game|GetPlayerCharacter 0))))))

(event EventBeginPlay
  (Utilities|FlowControl|Delay 1.0)
  (Utilities|FlowControl|DoOnce false
    (:Completed
      (if (Variables|Default|GetIsLeader?)
        (Variables|Default|SetLeader self)
        (CallFunction|SpawnHerd)))))

(event EventTick
  (params (DeltaSeconds :type Float%20%28single-precision%29)))

(fn ConstructionScript)