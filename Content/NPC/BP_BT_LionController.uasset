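; AI controller for the lion NPC that switches it between alert and calm states when it senses the first-person player.
; PawnSensing sight, or any heard noise (always attributed to player 0), sets blackboard alert and target keys and doubles walk speed.
; Retriggerable delays of twice the sensing interval clear alert and restore speed after stimuli stop, leaving the target key set.
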(event OnSeePawn(PawnSensing)
  (params (Pawn :type Pawn%20Object%20Reference))
  (bind _asfirst_person_character (Utilities|Casting|CastToFirstPersonCharacter Pawn))
  (CallFunction|SetCanSeePlayer? true _asfirst_person_character)
  (Utilities|FlowControl|RetriggerableDelay (* (Variables|/Script/AIModule.PawnSensingComponent|GetSensingInterval (Variables|Default|GetPawnSensing)) 2.0))
  (CallFunction|SetCanSeePlayer? false _asfirst_person_character))

(event OnHearNoise(PawnSensing)
  (params (Instigator :type Pawn%20Object%20Reference) (Location :type Vector%20%28by%20ref%29 :default "0, 0, 0") (Volume :type Float%20%28single-precision%29))
  (bind _asfirst_person_character (Utilities|Casting|CastToFirstPersonCharacter (Game|GetPlayerCharacter 0)))
  (CallFunction|SetCanSeePlayer? true _asfirst_person_character)
  (Utilities|FlowControl|RetriggerableDelay (* (Variables|/Script/AIModule.PawnSensingComponent|GetSensingInterval (Variables|Default|GetPawnSensing)) 2.0))
  (CallFunction|SetCanSeePlayer? false _asfirst_person_character))

(event EventBeginPlay)

(event EventTick
  (params (DeltaSeconds :type Float%20%28single-precision%29)))

(fn ConstructionScript)

(fn SetCanSeePlayer?
  (params (CanSee :type Boolean) (Player :type First%20Person%20Character%20Object%20Reference))
  (bind _self self)
  (bind _returnvalue (AI|GetBlackboard _self))
  (if CanSee
    (AI|Components|Blackboard|SetValueasBool _returnvalue (Utilities|Name|MakeLiteralName "ISAlert?") true)
    (AI|Components|Blackboard|SetValueasObject _returnvalue (Utilities|Name|MakeLiteralName "PlayerTarget") Player)
    (Variables|/Script/Engine.CharacterMovementComponent|SetMaxWalkSpeed (Variables|/Script/Engine.Character|GetCharacterMovement (.AsBP%20Lion%20Character (Utilities|Casting|CastToBP_LionCharacter (Pawn|GetControlledPawn self)))) 6e+02)
    (else
      (AI|Components|Blackboard|SetValueasBool _returnvalue (Utilities|Name|MakeLiteralName "ISAlert?") false)
      (Variables|/Script/Engine.CharacterMovementComponent|SetMaxWalkSpeed (Variables|/Script/Engine.Character|GetCharacterMovement (.AsBP%20Lion%20Character (Utilities|Casting|CastToBP_LionCharacter (Pawn|GetControlledPawn self)))) 3e+02))))